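; Blueprint function library of global getters for the SwordRay game's core framework objects.
; It returns the game mode, the first player controller, the controlled player character and that character's mesh anim instance, each cast to its project Blueprint class.
; The getters chain: the character comes from the controller's controlled pawn, and the anim Blueprint comes from the character.
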(fn `Get SRAnimBP`
  (returns (AsAnimBP :type "/Game/Blueprints/Character/ABP_PlayerCharacter Object Reference"))
  (bind _asabp_player_character (cast `/Game/Blueprints/Character/ABP_PlayerCharacter` (`SkeletalMeshComponent.GetAnimInstance` (`Character.Mesh` (`self.GetSRPlayer` null)))))
  (return _asabp_player_character))

(fn `GetGameModeBP`
  (returns (`As GameMode` :type "/Game/Blueprints/Common/BP_SwordRayGameModeBase Object Reference"))
  (bind _asbp_sword_ray_game_mode_base (cast `/Game/Blueprints/Common/BP_SwordRayGameModeBase` (`GameplayStatics.GetGameMode` null)))
  (return _asbp_sword_ray_game_mode_base))

(fn `GetPlayerControllerBP`
  (returns (`As PlayerController` :type "/Game/Blueprints/Character/BP_PlayerController Object Reference"))
  (bind _asbp_player_controller (cast `/Game/Blueprints/Character/BP_PlayerController` (`GameplayStatics.GetPlayerController` null)))
  (return _asbp_player_controller))

(fn `GetSRPlayer`
  (returns (AsPlayer :type "/Game/Blueprints/Character/BP_PlayerCharacter Object Reference"))
  (bind _asbp_player_character (cast `/Game/Blueprints/Character/BP_PlayerCharacter` (`Controller.K2_GetPawn` (`self.GetPlayerControllerBP` null))))
  (return _asbp_player_character))