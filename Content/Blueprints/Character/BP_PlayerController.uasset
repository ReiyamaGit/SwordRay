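; BP_PlayerController is the player controller that drives character movement and camera rotation from input.
; Look axes feed pitch and yaw, and Tick moves the pawn forward and sideways relative to camera yaw.
; Movement is gated by the animation Blueprint: it requires IsAttack to be false and CheckEnableRun to return IsRun as true.
; BeginPlay re-possesses the controlled pawn, and the left shoulder input only prints a debug string.
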(event `InputAction|LeftShalder`
  (params (Key :type "Key Structure"))
  (:`Pressed`
    (`KismetSystemLibrary.PrintString` "Hello")))

(event `InputAxis|LookUp`
  (params (AxisValue :type "Float (single-precision)"))
  (`self.AddPitchInput` AxisValue))

(event `InputAxis|RotateCamera`
  (params (AxisValue :type "Float (single-precision)"))
  (`self.AddYawInput` AxisValue))

(event `self.ReceiveBeginPlay`
  (`self.Possess` (`self.K2_GetPawn`)))

(event `self.ReceiveTick`
  (params (DeltaSeconds :type "Float (single-precision)"))
  (bind (_returnvalue_roll _returnvalue_pitch _returnvalue_yaw) (`KismetMathLibrary.BreakRotator` (`PlayerCameraManager.GetCameraRotation` (`self.PlayerCameraManager`))))
  (bind _returnvalue (`KismetMathLibrary.MakeRotator` 0.0 0.0 _returnvalue_yaw))
  ;[0.179 1 0.5114] 移動処理
  (bind _asabp_player_character (cast `/Game/Blueprints/Character/ABP_PlayerCharacter` (`/Game/Blueprints/Character/BP_SRFunctionLibrary.GetSRAnimInstance` (`/Game/Blueprints/Character/BP_SRFunctionLibrary.GetSRPlayer`))))
  (if (and (not (`/Game/Blueprints/Character/ABP_PlayerCharacter.IsAttack` _asabp_player_character)) (`self.CheckEnableRun`))
    (`Pawn.AddMovementInput` (`self.K2_GetPawn`) (`KismetMathLibrary.GetForwardVector` _returnvalue) (`self.GetInputAxisValue`) false)
    (`Pawn.AddMovementInput` (`self.K2_GetPawn`) (`KismetMathLibrary.GetRightVector` _returnvalue) (`self.GetInputAxisValue`) false)))

(fn `CheckEnableRun`
  (returns (bCanRun :type Boolean))
  (bind _asbp_player_character (cast `/Game/Blueprints/Character/BP_PlayerCharacter` (`self.K2_GetPawn`)))
  (bind _asabp_player_character (cast `/Game/Blueprints/Character/ABP_PlayerCharacter` (`SkeletalMeshComponent.GetAnimInstance` (`Character.Mesh` _asbp_player_character))))
  (return (`/Game/Blueprints/Character/ABP_PlayerCharacter.IsRun` _asabp_player_character)))

(fn `UserConstructionScript`)