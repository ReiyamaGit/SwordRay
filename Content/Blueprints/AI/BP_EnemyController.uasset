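; Enemy AI controller that runs the BT_Enemy behavior tree on possess and feeds perception results into its Blackboard.
; Sensing a Player-tagged actor cancels the line-of-sight timer and writes HasLineOfSight and EnemyActor immediately.
; Any other perception update starts a one-shot timer that writes the same keys on expiry.
; As wired, both paths set HasLineOfSight false and pass no object to EnemyActor.
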(event `self.ReceivePossess`
  (params (PossessedPawn :type "Pawn Object Reference"))
  (`self.RunBehaviorTree` "/Game/Blueprints/AI/BT_Enemy.BT_Enemy"))

(event `self.AIPerception.OnTargetPerceptionUpdated`
  (params (Actor :type "Actor Object Reference") (Stimulus :type "AIStimulus Structure"))
  (if (and (`self.ActorHasTag` Actor "Player") (`.bSuccessfullySensed` (break `AIStimulus` Stimulus)))
    (`KismetSystemLibrary.K2_ClearAndInvalidateTimerHandle` (`self.EnemyTimer`))
    (`BlackboardComponent.SetValueAsBool` (`self.Blackboard`) (`self.HasLineOfSight`) false)
    (`BlackboardComponent.SetValueAsObject` (`self.Blackboard`) (`self.EnemyActor`) null)
    (else
      (bind _returnvalue (`KismetSystemLibrary.K2_SetTimerDelegate` (delegate `StartEnemyTimer`) (`self.LineOfSightTimer`)))
      (set `self.EnemyTimer` _returnvalue))))

(event `StartEnemyTimer`
  (`BlackboardComponent.SetValueAsBool` (`self.Blackboard`) (`self.HasLineOfSight`) false)
  (`BlackboardComponent.SetValueAsObject` (`self.Blackboard`) (`self.EnemyActor`) null))

(fn `UserConstructionScript`)